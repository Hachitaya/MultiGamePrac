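; Base killer character Blueprint that attacks survivors, with the camera boom snapped to the head socket and yaw following the controller.
; Request/response event pairs hide the spotlight at BeginPlay and play the attack montage on input.
; AttackSurvivors, not called in this graph, damages survivors in a sphere overlap at AttackPoint and draws a debug sphere.
; GetStun disables player-zero input until a timer calls NoStun.
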(event Custom|ReqSetVis
  (CallFunction|ResSetVis))

(event Custom|ResSetVis
  (Development|SetHiddeninGame (Variables|Default|GetSpotLight) true false))

(event Custom|ReqAttack
  (CallFunction|ResAttack))

(event Custom|ResAttack
  (Animation|PlayAnimMontage "/Game/TotalAnimAssets/BossAnimationsPack/Animations/AttackMontages/BossSingleAttack_Montage.BossSingleAttack_Montage" 1.0 "NoDelay"))

(event EventBeginPlay
  (CallFunction|ReqSetVis))

(event Input|ActionEvents|InputActionAttack
  (params (Key :type Key%20Structure :default "None"))
  (:Pressed
    (CallFunction|ReqAttack)))

(fn ConstructionScript
  (|CallParentFunction)
  (Variables|Default|SetbUseControllerRotationYaw true)
  (Variables|/Script/Engine.CharacterMovementComponent|SetbOrientRotationToMovement (Variables|Character|GetCharacterMovement) false)
  (Transformation|AttachComponentToComponent (Variables|Default|GetCameraBoom) (Variables|Character|GetMesh) "HeadSocket" "SnapToTarget" "SnapToTarget" "SnapToTarget" true))

(fn AttackSurvivors
  (Rendering|Debug|DrawDebugSphere (Transformation|GetWorldLocation (Variables|Default|GetAttackPoint)) 1e+02 12 "(R=1.000000,G=0.090570,B=0.000000,A=1.000000)" 1e+01 1.0)
  (bind _outactors (Collision|SphereOverlapActors (Transformation|GetWorldLocation (Variables|Default|GetAttackPoint)) 1e+02 (Utilities|Array|MakeArray "ObjectTypeQuery3") "/Game/DBD/Blueprints/BP_SurvivorBase.BP_SurvivorBase_C"))
  (for _array_element _outactors
    (Game|Damage|ApplyDamage _array_element (Variables|Default|GetBaseDamage) 0 (Game|Player|GetPlayerPawn 0))))

(fn GetStun
  (Input|DisableInput (Game|GetPlayerController 0))
  (Utilities|Time|SetTimerbyFunctionName 0 "NoStun" 5.0))

(fn NoStun
  (Input|EnableInput (Game|GetPlayerController 0)))