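; Buff component, apparently work in progress, that tracks active buffs in an array and times their removal.
; ApplyBuff adds unique entries, while Tick compares the array to its previous snapshot, always using the DT_Buff "Buff1" row as the changed buff.
; Growth triggers activation and a Delay-based removal after the row's duration; other changes trigger deactivation.
; Activate and Deactivate only print, no target character is passed from Tick, and cooldown is an empty stub.
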(event Custom|SetDuration
  (params (ST_Buff :type ST%20Buff%20Structure) (Duration :type Float%20%28single-precision%29))
  (Utilities|FlowControl|Delay Duration)
  (CallFunction|RemoveBuff (Variables|Default|GetBuffArray) ST_Buff))

(event EventTick
  (params (DeltaSeconds :type Float%20%28single-precision%29))
  (bind _returnvalue (Utilities|GetDataTableRow "/Game/DBD/Data/DT_Buff.DT_Buff" "Buff1")
    (:then
      (CallFunction|CheckBuff (Variables|Default|GetBuffArray) _returnvalue))))

(event EventBeginPlay)

(fn ApplyBuff
  (params (ST_Buff :type ST%20Buff%20Structure) (TargetCharacter :type Character%20Object%20Reference))
  (Utilities|Array|AddUnique (Variables|Default|GetBuffArray) ST_Buff))

(fn CheckBuff
  (params (ActiveBuffArray :type Array%20of%20ST%20Buff%20Structures) (ST_Buff :type ST%20Buff%20Structure) (TargetCharacter :type Character%20Object%20Reference))
  (if (not (Utilities|Array|Identical ActiveBuffArray (Variables|Default|GetBeforeBuffArray)))
    (if (> (Utilities|Array|Length ActiveBuffArray) (Utilities|Array|Length (Variables|Default|GetBeforeBuffArray)))
      (CallFunction|ActivateBuff (.st_state ST_Buff) 0.0 TargetCharacter)
      (CallFunction|SetBuffDuration ST_Buff (.duration ST_Buff))
      (else
        (CallFunction|DeactivateBuff (.st_state ST_Buff) (.cooldowntime ST_Buff) TargetCharacter)))
    (Variables|Default|SetBeforeBuffArray ActiveBuffArray)))

(fn RemoveBuff
  (params (ActiveBuffArray :type Array%20of%20ST%20Buff%20Structures) (ST_Buff :type ST%20Buff%20Structure) (Char :type Character%20Object%20Reference))
  (Utilities|Array|RemoveItem ActiveBuffArray ST_Buff))

(fn ActivateBuff
  (params (ST_State :type ST%20State%20Structure) (Duration :type Float%20%28single-precision%29) (TargetCharacter :type Character%20Object%20Reference))
  (Development|PrintString "Activated" true true "(R=1.000000,G=0.008313,B=0.000000,A=1.000000)"))

(fn DeactivateBuff
  (params (ST_State :type ST%20State%20Structure) (CoolDowntime :type Float%20%28single-precision%29) (TargetCharacter :type Character%20Object%20Reference))
  (Development|PrintString "Deactivated" true true "(R=1.000000,G=0.008313,B=0.000000,A=1.000000)"))

(fn SetBuffCoolDownTime)

(fn SetBuffDuration
  (params (ST_Buff :type ST%20Buff%20Structure) (Duration :type Float%20%28single-precision%29))
  (CallFunction|SetDuration ST_Buff Duration))

(fn RemoveBuffReapeter
  (params (ST_Buff :type ST%20Buff%20Structure) (Duration :type Float%20%28single-precision%29)))