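; Survivor actor component that holds a three-slot skill loadout, seeded from DT_Skill and mirrored to the HUD skill list.
; Activating a skill triggers the UI cooldown event and, if it is not cooling, applies its buff through BP_BuffComponent and queues it.
; A 0.1-second timer diffs the cooling queue against a snapshot to set per-ID cooldown flags and start countdowns.
; Tick decrements those countdowns and removes expired skills.
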(event EventBeginPlay
  ;[1 1 1] 코멘트
  (bind _asbp_survivor_base (Utilities|Casting|CastToBP_SurvivorBase (Components|GetOwner)))
  (bind _output_get (Variables|Default|SetOwnCharacter _asbp_survivor_base))
  (Variables|Default|SetBuffComponent (Actor|GetComponentbyClass _output_get "/Game/DBD/Data/BP_BuffComponent.BP_BuffComponent_C"))
  (bind _ashd_dbdhudclass (Utilities|Casting|CastToHD_DBDHUDClass (HUD|GetHUD (Game|GetPlayerController 0))))
  (Variables|Default|SetUserSkillList (Variables|/Game/DBD/Widget/UMG_HUD.UMG_HUD_C|GetUMG_SkillList (Variables|/Game/DBD/Blueprints/GameBase/HD_DBDHUDClass.HD_DBDHUDClass_C|GetHUDWidget _ashd_dbdhudclass)))
  (기본/디폴트|InitSkillArray)
  (기본/디폴트|UpdateSkillList)
  (기본/디폴트|CheckCoolingSkill)
  (Utilities|Time|SetTimerbyFunctionName 0 "CheckCoolingSkill" 0.1 true))

(event EventTick
  (params (DeltaSeconds :type Float%20%28single-precision%29))
  (기본/디폴트|CheckCoolTimer DeltaSeconds))

(fn ActivateSkill
  (params (SkillArrayIndex :type Integer))
  (bind _settingskillarray (Variables|Default|GetSettingSkillArray))
  (bind _output (Utilities|Array|Get(acopy) _settingskillarray SkillArrayIndex))
  (bind (_skillid _skillname _st_buff _icon _isactive) (Utilities|Struct|BreakST_Skill _output))
  (if _isactive
    (Default|CoolDownEvent (Variables|Default|GetUserSkillList) SkillArrayIndex)
    (if (not (Utilities|Array|Get(acopy) (Variables|Default|GetCoolingSkillArray) _skillid))
      (Default|ApplyBuff (Variables|Default|GetBuffComponent) _st_buff)
      (기본/디폴트|AddCoolingSkillArray _output))))

(fn SetIndex
  (params (CurrentSelectedUserSkillIndex :type Integer))
  (Variables|Default|SetCurrentSelectedUserSkillIndex CurrentSelectedUserSkillIndex))

(fn ChangeSkillArray
  (params (ST_Skill :type ST%20Skill%20Structure%20%28by%20ref%29))
  (Utilities|Array|SetArrayElem (Variables|Default|GetSettingSkillArray) (Variables|Default|GetCurrentSelectedUserSkillIndex) ST_Skill)
  (기본/디폴트|UpdateSkillList))

(fn InitSkillArray
  (for _index (range 0 2)
    (bind _returnvalue (Utilities|GetDataTableRow "/Game/DBD/Data/DT_Skill.DT_Skill" "1")
      (:then
        (Utilities|Array|Add (Variables|Default|GetSettingSkillArray) _returnvalue)))))

(fn UpdateSkillList
  (bind _userskilllist (Variables|Default|GetUserSkillList))
  (Utilities|IsValid _userskilllist
    (:Is%20Valid
      (Default|ClearList _userskilllist)
      (for _array_element (Variables|Default|GetSettingSkillArray)
        (Default|AddSkillSlot (Variables|Default|GetUserSkillList) (.SkillName (Utilities|Struct|BreakST_Skill _array_element)))))))

(fn AddCoolingSkillArray
  (params (ST_Skill :type ST%20Skill%20Structure))
  (bind _output_get (Variables|Default|SetST_Skill_Temp ST_Skill))
  (Utilities|Array|Add (Variables|Default|GetCoolSkillArray) _output_get))

(fn CheckCoolingSkill
  (if (not (Utilities|Array|Identical (Variables|Default|GetCoolSkillArray) (Variables|Default|GetBeforeCoolingSkillArray)))
    (if (> (Utilities|Array|Length (Variables|Default|GetCoolSkillArray)) (Utilities|Array|Length (Variables|Default|GetBeforeCoolingSkillArray)))
      (기본/디폴트|StartSkillCoolDown)
      (else
        (기본/디폴트|EndSkillCookDown)))
    (Variables|Default|SetBeforeCoolingSkillArray (Variables|Default|GetCoolSkillArray))))

(fn RemoveCoolingSkill
  (params (ST_Skill :type ST%20Skill%20Structure))
  (bind _output_get (Variables|Default|SetST_Skill_Temp ST_Skill))
  (Utilities|Array|RemoveItem (Variables|Default|GetCoolSkillArray) _output_get))

(fn StartSkillCoolDown
  (bind _st_skill_temp (Variables|Default|GetST_Skill_Temp))
  (bind (_skillid _skillname _st_buff) (Utilities|Struct|BreakST_Skill _st_skill_temp))
  (Utilities|Array|SetArrayElem (Variables|Default|GetCoolingSkillArray) _skillid true)
  (기본/디폴트|AddCoolTimer (.cooldowntime _st_buff)))

(fn EndSkillCookDown
  (Utilities|Array|SetArrayElem (Variables|Default|GetCoolingSkillArray) (.SkillID (Utilities|Struct|BreakST_Skill (Variables|Default|GetST_Skill_Temp))) false))

(fn AddCoolTimer
  (params (CoolTime :type Float%20%28single-precision%29%20%28by%20ref%29))
  (Utilities|Array|Add (Variables|Default|GetCoolTimeArray) CoolTime))

(fn CheckCoolTimer
  (params (DelatSecond :type Float%20%28single-precision%29))
  (bind _cooltimearray (Variables|Default|GetCoolTimeArray))
  (LocalVariables|SetLength (- (Utilities|Array|Length (Variables|Default|GetCoolTimeArray)) 1))
  (Utilities|FlowControl|Sequence
    (:then_0
      (for _index (range 0 (LocalVariables|GetLength))
        (Utilities|Array|SetArrayElem _cooltimearray _index (- (Utilities|Array|Get(acopy) _cooltimearray _index) DelatSecond))
        (Development|PrintString (Utilities|String|ToString(Float) (- (Utilities|Array|Get(acopy) _cooltimearray _index) DelatSecond)) true true "(R=0.000000,G=0.660000,B=1.000000,A=1.000000)" 0.0)))
    (:then_1
      (for _index_2 (range 0 (LocalVariables|GetLength))
        (if (and (< (Utilities|Array|Get(acopy) (Variables|Default|GetCoolTimeArray) _index_2) 0.0) (> (Utilities|Array|Get(acopy) (Variables|Default|GetCoolTimeArray) _index_2) -1e+02))
          (기본/디폴트|RemoveCoolingSkill (Utilities|Array|Get(acopy) (Variables|Default|GetCoolSkillArray) _index_2))
          (Utilities|Array|RemoveIndex (Variables|Default|GetCoolTimeArray) _index_2))))))