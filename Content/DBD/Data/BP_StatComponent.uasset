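; Stat component for survivor characters that keeps base, additional and result values in parallel arrays indexed by the EStat enum.
; On BeginPlay it fills base values from DT_BasicStat, zeroes additional values and copies base into result.
; IncreaseStat and DecreaseStat add or subtract a stat's additional value on its current result.
; Table length comes from probing numeric row names from zero until one is missing.
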(event EventBeginPlay
  (bind _asbp_survivor_base (Utilities|Casting|CastToBP_SurvivorBase (Components|GetOwner)))
  (Variables|Default|SetOwnerCharacter _asbp_survivor_base)
  (CallFunction|InitStatArray)
  (Variables|Default|SetResultStatArray (Variables|Default|GetBaseStatArray)))

(fn IncreaseStat
  (params (E_Stat :type E_Stat%20Enum :default "NewEnumerator0"))
  (bind _output_get (LocalVariables|SetIndex (Math|Conversions|ToInteger(Byte) E_Stat)))
  (Utilities|Array|SetArrayElem (Variables|Default|GetResultStatArray) _output_get (+ (CallFunction|GetResultStat E_Stat) (CallFunction|GetAdditionalStat E_Stat))))

(fn DecreaseStat
  (params (E_Stat :type E_Stat%20Enum :default "NewEnumerator0"))
  (bind _output_get (LocalVariables|SetIndex (Math|Conversions|ToInteger(Byte) E_Stat)))
  (Utilities|Array|SetArrayElem (Variables|Default|GetResultStatArray) _output_get (- (CallFunction|GetResultStat E_Stat) (CallFunction|GetAdditionalStat E_Stat))))

(fn GetResultStat
  (params (E_Stat :type E_Stat%20Enum :default "NewEnumerator0"))
  (return (Utilities|Array|Get(acopy) (Variables|Default|GetResultStatArray) (Math|Conversions|ToInteger(Byte) E_Stat))))

(fn GetBaseStat
  (params (E_Stat :type E_Stat%20Enum :default "NewEnumerator0"))
  (return (Utilities|Array|Get(acopy) (Variables|Default|GetBaseStatArray) (Math|Conversions|ToInteger(Byte) E_Stat))))

(fn GetAdditionalStat
  (params (E_Stat :type E_Stat%20Enum :default "NewEnumerator0"))
  (return (Utilities|Array|Get(acopy) (Variables|Default|GetAdditionalStatArray) (Math|Conversions|ToInteger(Byte) E_Stat))))

(fn SetBaseStat
  (params (E_Stat :type E_Stat%20Enum :default "NewEnumerator0") (Value :type Float%20%28single-precision%29))
  (Utilities|Array|SetArrayElem (Variables|Default|GetBaseStatArray) (Math|Conversions|ToInteger(Byte) E_Stat) Value true))

(fn SetAdditionalStat
  (params (E_Stat :type E_Stat%20Enum :default "NewEnumerator0") (Value :type Float%20%28single-precision%29))
  (Utilities|Array|SetArrayElem (Variables|Default|GetAdditionalStatArray) (Math|Conversions|ToInteger(Byte) E_Stat) Value true))

(fn SetResultStat
  (params (E_Stat :type E_Stat%20Enum :default "NewEnumerator0") (Value :type Float%20%28single-precision%29))
  (Utilities|Array|SetArrayElem (Variables|Default|GetResultStatArray) (Math|Conversions|ToInteger(Byte) E_Stat) Value))

(fn InitStatArray
  (for _index (range 0 (CallFunction|GetDataTableLength "/Game/DBD/Data/DT_BasicStat.DT_BasicStat"))
    (bind _returnvalue (Utilities|GetDataTableRow "/Game/DBD/Data/DT_BasicStat.DT_BasicStat" (Utilities|String|StringToName (Utilities|String|ToString(Integer) _index)))
      (:then
        (CallFunction|SetBaseStat (.Stat (Utilities|Struct|BreakST_State _returnvalue)) (.BaseValue (Utilities|Struct|BreakST_State _returnvalue)))
        (CallFunction|SetAdditionalStat (.Stat (Utilities|Struct|BreakST_State _returnvalue)) 0.0)))))

(fn GetDataTableLength
  (params (DataTable :type Data%20Table%20Object%20Reference))
  (while true
    (bind _returnvalue (Utilities|GetDataTableRow DataTable (Utilities|String|StringToName (Utilities|String|ToString(Integer) (LocalVariables|GetCurrentLen))))
      (:then
        (Math|Integer|IncrementInt (LocalVariables|GetCurrentLen)
          (:%20%20
            (LocalVariables|SetData _returnvalue))))
      (:RowNotFound
        (return (LocalVariables|GetCurrentLen))))))