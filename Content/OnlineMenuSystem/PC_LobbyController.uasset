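; Player controller for the online lobby that shows each player a lobby menu and enables the mouse cursor.
; On BeginPlay, CreateMenus uses an authority check to create the host screen on authority or the client screen on remote, storing it as LobbyWidget.
; It then switches player 0 to UI-only input.
; On authority, BeginPlay also sets the game mode's default pawn class to BP_SurvivorBase.
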(event Custom|CreateMenus
  (Networking|SwitchHasAuthority
    (:Authority
      (bind _returnvalue (UserInterface|CreateWidget "/Game/OnlineMenuSystem/UMG/UMG_LobbyHostScreen.UMG_LobbyHostScreen_C"))
      (bind _output_get (Variables|Default|SetLobbyWidget _returnvalue))
      (UserInterface|Viewport|AddtoViewport _output_get 0))
    (:Remote
      (bind _returnvalue_2 (UserInterface|CreateWidget "/Game/OnlineMenuSystem/UMG/UMG_ClientScreen.UMG_ClientScreen_C"))
      (bind _output_get_2 (Variables|Default|SetLobbyWidget _returnvalue_2))
      (UserInterface|Viewport|AddtoViewport _output_get_2 0)))
  (Input|SetInputModeUIOnly (Game|GetPlayerController 0) 0 "DoNotLock"))

(event EventBeginPlay
  (CallFunction|CreateMenus)
  (Networking|SwitchHasAuthority
    (:Authority
      (Variables|/Script/Engine.GameModeBase|SetDefaultPawnClass (Game|GetGameMode) "/Game/DBD/Blueprints/BP_SurvivorBase.BP_SurvivorBase_C"))))

(fn ConstructionScript
  (Variables|Default|SetbShowMouseCursor true))